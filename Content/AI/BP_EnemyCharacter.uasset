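; BP_EnemyCharacter is an AI enemy character that reports player detection to its AI controller's Blackboard.
; Its AIPerception target update event proceeds only when the sensed actor is BP_MyCharacter and its controller is BP_EnemyAIController.
; A successful sense sets the player-detected key and stores the player as target actor; losing the sense clears both.
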(event `self.AIPerception.OnTargetPerceptionUpdated`
  (params (Actor :type "Actor Object Reference") (Stimulus :type "AIStimulus Structure"))
  ; 인지를 하는 순간 호출 되는 이벤트
  (bind _asbp_my_character (cast `/Game/Blueprints/BP_MyCharacter` Actor))
  (bind _asbp_enemy_aicontroller (cast `/Game/AI/BP_EnemyAIController` (`self.GetController`)))
  (if Stimulus_bSuccessfullySensed
    (bind _returnvalue (`AIBlueprintHelperLibrary.GetBlackboard` _asbp_enemy_aicontroller))
    ; Blackboard의 PlayerDetected(True)/TargetActor(Player) 변수값 할당
    (`BlackboardComponent.SetValueAsBool` _returnvalue (`self.PlayerDetectedKey`) true)
    (`BlackboardComponent.SetValueAsObject` _returnvalue (`self.TargetActorKey`) _asbp_my_character)
    (else
      (bind _returnvalue_2 (`AIBlueprintHelperLibrary.GetBlackboard` _asbp_enemy_aicontroller))
      ; Blackboard의 PlayerDetected(False)/TargetActor(nullptr) 변수값 할당
      (`BlackboardComponent.SetValueAsBool` _returnvalue_2 (`self.PlayerDetectedKey`) false)
      (`BlackboardComponent.SetValueAsObject` _returnvalue_2 (`self.TargetActorKey`) null))))

(fn `UserConstructionScript`)